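; Collectible crystal actor that gets drawn into the player and disappears when an actor overlaps it, with no filter on which actor.
; On overlap it stores its starting location and scale, then plays a timeline with separate tracks for pull, shrink and light.
; Each update lerps it toward player pawn 0's current location, shrinks it to zero and sets point light intensity, then the actor destroys itself on finish.
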(event `self.ReceiveActorBeginOverlap`
  (params (OtherActor :type "Actor Object Reference"))
  (if true
    (bind _output_get (`self.F Get Object Start Location`))
    (bind _output_get_2 (`self.F_GetObjectStartScale`))
    (bind (_direction _succ _smol _lightintensity) (`Timeline|TL_BlendAlpha`)
      (:`Update`
        (`self.F Move Object to Player Pawn` _output_get (`self.K2_GetActorLocation` (`GameplayStatics.GetPlayerPawn` 0)) _succ)
        (`self.F Set New Object Scale` _output_get_2 _smol)
        (`self.LightIntensity` _lightintensity))
      (:`Finished`
        (`self.K2_DestroyActor`)))))

(fn `F Get Object Start Location`
  (returns (Output_Get :type "Vector Structure"))
  (bind _output_get (set `self.LerpStartLocation` (`self.K2_GetActorLocation`)))
  (return _output_get))

(fn `F Move Object to Player Pawn`
  (params (A :type "Vector Structure") (B :type "Vector Structure") (Alpha :type "Float (double-precision)"))
  (`self.K2_SetActorLocation` (`KismetMathLibrary.VLerp` A B Alpha)))

(fn `F Set New Object Scale`
  (params (A :type "Vector Structure") (Alpha :type "Float (double-precision)"))
  (`self.SetActorScale3D` (`KismetMathLibrary.VLerp` A (0.0 0.0 0.0) Alpha)))

(fn `F_GetObjectStartScale`
  (returns (Output_Get :type "Vector Structure"))
  (bind _output_get (set `self.LerpStartScale` (`self.GetActorScale3D`)))
  (return _output_get))

(fn `Light Intensity`
  (params (NewIntensity :type "Float (double-precision)"))
  (`LightComponent.SetIntensity` (`self.PointLight`) NewIntensity))

(fn `LightIntensity`
  (params (NewIntensity :type "Float (double-precision)"))
  (`LightComponent.SetIntensity` (`self.PointLight`) NewIntensity))

(fn `UserConstructionScript`)