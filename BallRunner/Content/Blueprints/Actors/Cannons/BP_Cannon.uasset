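; Cannon actor that fires automatically on a repeating cycle by spawning an actor at its Projectile component's location and rotation.
; BeginPlay waits a short random time, then a two-second Delay precedes each shot.
; Each shot plays a timeline that moves the Cannon component along its relative Y axis.
; The timeline's Update loops back into that Delay, so firing repeats without Tick.
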(event `self.ReceiveBeginPlay`
  (`KismetSystemLibrary.Delay` (`KismetMathLibrary.RandomFloatInRange` 0.1 1.0))
  (`KismetSystemLibrary.Delay` 2.0 :!label _label)
  (`|SpawnActorFromClass` "/Game/Blueprints/Actors/Projectiles/BP_Projectile_1.BP_Projectile_1_C" (`KismetMathLibrary.MakeTransform` (`SceneComponent.K2_GetComponentLocation` (`self.Projectile`)) (`SceneComponent.K2_GetComponentRotation` (`self.Projectile`))) "Undefined" "OverrideRootScale" null null)
  (bind (_direction _cannon) (`Timeline|Timeline_0` :!via `PlayFromStart`)
    (:`Update`
      (`SceneComponent.K2_SetRelativeLocation` (`self.Cannon`) (`KismetMathLibrary.MakeVector` 0.0 _cannon) false false)
      (goto _label))))

(event `self.ReceiveTick`
  (params (DeltaSeconds :type "Float (single-precision)")))

(fn `UserConstructionScript`)